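; Drivable pickup vehicle pawn with enter/exit support, a handbrake and a toggleable back door.
; Input feeds throttle, steering and handbrake to VehicleMovement, and yaws the SpringArm camera; vertical look applies zero rotation.
; Box overlap flags the ALS character as ready to enter and passes it this vehicle; F spawns a new character at Spawn1 and possesses it.
; A FlipFlop plays or reverses the BackDoor timeline, which drives BackDoorAngle.
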(event OnComponentBeginOverlap(Box)
  (params (OverlappedComponent :type Primitive%20Component%20Object%20Reference) (OtherActor :type Actor%20Object%20Reference) (OtherComp :type Primitive%20Component%20Object%20Reference) (OtherBodyIndex :type Integer) (bFromSweep :type Boolean) (SweepResult :type Hit%20Result%20Structure%20%28by%20ref%29))
  ;[1 1 1] Detetar se foi o jogador a dar overlap na Collison Box e se sim passar uma referencia do veiculo para a blueprint do jogador
  (bind _asals_anim_man_character_bp (Utilities|Casting|CastToALS_AnimMan_CharacterBP OtherActor))
  (Variables|/Game/AdvancedLocomotionV4/Blueprints/CharacterLogic/ALS_AnimMan_CharacterBP.ALS_AnimMan_CharacterBP_C|SetReadyToEnterVehicle? _asals_anim_man_character_bp true)
  (Variables|/Game/AdvancedLocomotionV4/Blueprints/CharacterLogic/ALS_AnimMan_CharacterBP.ALS_AnimMan_CharacterBP_C|SetVehicleToEnter _asals_anim_man_character_bp self))

(event OnComponentEndOverlap(Box)
  (params (OverlappedComponent :type Primitive%20Component%20Object%20Reference) (OtherActor :type Actor%20Object%20Reference) (OtherComp :type Primitive%20Component%20Object%20Reference) (OtherBodyIndex :type Integer))
  ;[1 1 1] Detetar se foi o jogador a dar overlap na Collison Box e se sim passar uma referencia do veiculo para a blueprint do jogador
  (bind _asals_anim_man_character_bp (Utilities|Casting|CastToALS_AnimMan_CharacterBP OtherActor))
  (Variables|/Game/AdvancedLocomotionV4/Blueprints/CharacterLogic/ALS_AnimMan_CharacterBP.ALS_AnimMan_CharacterBP_C|SetReadyToEnterVehicle? _asals_anim_man_character_bp false))

(event EventBeginPlay)

(event Collision|EventActorBeginOverlap
  (params (OtherActor :type Actor%20Object%20Reference)))

(event EventTick
  (params (DeltaSeconds :type Float%20%28single-precision%29)))

(event Input|ActionEvents|InputActionHandBrake
  (params (Key :type Key%20Structure :default "None"))
  (bind _vehiclemovement (Variables|Default|GetVehicleMovement))
  ;[1 1 1] Handbrake
  (:Pressed
    (Class|WheeledVehicleMovementComponent|SetHandbrakeInput _vehiclemovement true))
  (:Released
    (Class|WheeledVehicleMovementComponent|SetHandbrakeInput _vehiclemovement false)))

(event Input|ActionEvents|InputActionBackDoorTrigger
  (params (Key :type Key%20Structure :default "None"))
  ;[1 1 1] Door functionality
  (:Pressed
    (Utilities|FlowControl|FlipFlop
      (:A
        (bind _door_angle (Timeline|BackDoor Play)
          (:Update
            (Variables|Default|SetBackDoorAngle _door_angle))))
      (:B
        (Timeline|BackDoor Reverse)))))

(event Input|AxisEvents|InputAxisLookUp/Down
  (params (AxisValue :type Float%20%28single-precision%29))
  ;[1 1 1] Camera Look Around
  (Transformation|AddRelativeRotation (Variables|Default|GetSpringArm) (Math|Rotator|MakeRotator 0.0 0.0 0.0) false false))

(event Input|AxisEvents|InputAxisLookLeft/Right
  (params (AxisValue :type Float%20%28single-precision%29))
  ;[1 1 1] Camera Look Around
  (Transformation|AddRelativeRotation (Variables|Default|GetSpringArm) (Math|Rotator|MakeRotator 0.0 0.0 AxisValue) false false))

(event Input|AxisEvents|InputAxisMoveForward/Backwards
  (params (AxisValue :type Float%20%28single-precision%29))
  ;[1 1 1] Throttle and Steering
  (Class|WheeledVehicleMovementComponent|SetThrottleInput (Variables|Default|GetVehicleMovement) AxisValue))

(event Input|AxisEvents|InputAxisMoveRight/Left
  (params (AxisValue :type Float%20%28single-precision%29))
  ;[1 1 1] Throttle and Steering
  (Class|WheeledVehicleMovementComponent|SetSteeringInput (Variables|Default|GetVehicleMovement) AxisValue))

(event Input|KeyboardEvents|F
  (params (Key :type Key%20Structure :default "None"))
  ;[1 1 1] Sair do carro
  (:Pressed
    (bind _returnvalue (Game|SpawnActorfromClass "/Game/AdvancedLocomotionV4/Blueprints/CharacterLogic/ALS_AnimMan_CharacterBP.ALS_AnimMan_CharacterBP_C" (Math|Transform|MakeTransform (Transformation|GetWorldLocation (Variables|Default|Getspawn1)) "0, 0, 0" "1,1,1") "AdjustIfPossibleButAlwaysSpawn" 0 0))
    (Pawn|Possess (Game|GetPlayerController 0) _returnvalue)))

(fn ConstructionScript)